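; Player controller for a grid-based city builder that forwards camera input to the CameraContoller pawn and runs building placement.
; In placement mode it spawns a preview actor, which follows a cursor line trace each Tick, snapped to the GridManager's plots.
; Left click spawns valid buildings, marks cells occupied, registers roads and charges costs through the game mode.
; Actor tags then drive game state updates and end placement mode.
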(event `PlacementData`
  (params (placeableActorType :type "/Game/GameObjects/Objects/Placeable_Base_asset Class Reference") (BuildingMode :type "/Game/GameObjects/GridManager/BuildingTypeEnum Enum" :default "NewEnumerator3"))
  (bind _placeableactor (`self.placeableActor`))
  ;[1 1 1] Updates building you are placeing
  (set `self.placeableActorType` placeableActorType)
  (bind _output_get (set `self.PlaceableBuildingType` BuildingMode))
  (if (`|EnumEquality` _output_get "NewEnumerator3")
    (`self.SetPlacementModeEnabled` false)
    (else
      (`/Engine/EditorBlueprintResources/StandardMacros.IsValid` _placeableactor
        (:`Is Valid`
          (`self.K2_DestroyActor` _placeableactor))
        (:`Is Not Valid`
          _))
      (`self.UpdatesBuildingType`)
      (`self.SetPlacementModeEnabled` true))))

(event `InputAxis|CamOrbit`
  (params (AxisValue :type "Float (single-precision)"))
  ;[1 1 1] calls camera orbit
  (bind _ascamera_contoller (cast `/Game/Character/CameraContoller` (`self.K2_GetPawn`)))
  (`/Game/Character/CameraContoller.CamOrbit` _ascamera_contoller AxisValue))

(event `InputAxis|MoveForwardBack`
  (params (AxisValue :type "Float (single-precision)"))
  ;[1 1 1] calls function to move camera left/right up/down
  (bind _ascamera_contoller (cast `/Game/Character/CameraContoller` (`self.K2_GetPawn`)))
  (`/Game/Character/CameraContoller.MoveForwardBack` _ascamera_contoller AxisValue))

(event `InputAxis|MoveLeftRight`
  (params (AxisValue :type "Float (single-precision)"))
  ;[1 1 1] calls function to move camera left/right up/down
  (bind _ascamera_contoller (cast `/Game/Character/CameraContoller` (`self.K2_GetPawn`)))
  (`/Game/Character/CameraContoller.MoveLeftRight` _ascamera_contoller AxisValue))

(event `InputAction|CameraZoomIn`
  (params (Key :type "Key Structure"))
  ;[1 1 1] calls camra zoom in/out
  (:`Pressed`
    (bind _ascamera_contoller (cast `/Game/Character/CameraContoller` (`self.K2_GetPawn`)))
    (`/Game/Character/CameraContoller.CameraZoom` _ascamera_contoller -1.0)))

(event `InputAction|CameraZoomOut`
  (params (Key :type "Key Structure"))
  ;[1 1 1] calls camra zoom in/out
  (:`Pressed`
    (bind _ascamera_contoller (cast `/Game/Character/CameraContoller` (`self.K2_GetPawn`)))
    (`/Game/Character/CameraContoller.CameraZoom` _ascamera_contoller 1.0)))

(event `InputAxis|CameraPitch`
  (params (AxisValue :type "Float (single-precision)"))
  ;[1 1 1] calls function for camera pitch
  (bind _ascamera_contoller (cast `/Game/Character/CameraContoller` (`self.K2_GetPawn`)))
  (`/Game/Character/CameraContoller.CameraPitch` _ascamera_contoller AxisValue))

(event `InputAction|MouseRightClick`
  (params (Key :type "Key Structure"))
  ;[1 1 1] calls function for camera to be controled with right click and mouse
  (:`Pressed`
    (set `self.RightButtonPressed` true))
  (:`Released`
    (set `self.RightButtonPressed` false)))

(event `InputAxis|MouseY`
  (params (AxisValue :type "Float (single-precision)"))
  ;[1 1 1] calls function for camera to be controled with right click and mouse
  (if (`self.RightButtonPressed`)
    (bind _ascamera_contoller (cast `/Game/Character/CameraContoller` (`self.K2_GetPawn`)))
    (`/Game/Character/CameraContoller.CameraPitch` _ascamera_contoller AxisValue)))

(event `InputAxis|MouseX`
  (params (AxisValue :type "Float (single-precision)"))
  ;[1 1 1] calls function for camera to be controled with right click and mouse
  (if (`self.RightButtonPressed`)
    (bind _ascamera_contoller (cast `/Game/Character/CameraContoller` (`self.K2_GetPawn`)))
    (`/Game/Character/CameraContoller.CamOrbit` _ascamera_contoller AxisValue)))

(event `self.ReceiveBeginPlay`
  (`self.SetPlacementModeEnabled` true)
  (`GameplayStatics.GetActorOfClass` null))

(event `self.ReceiveTick`
  (params (DeltaSeconds :type "Float (single-precision)"))
  (if (`self.placementModeActive`)
    (`self.UpdatePlacement`)))

(event `InputAction|MouseLeftClick`
  (params (Key :type "Key Structure"))
  (:`Pressed`
    (if (`self.placementModeActive`)
      (`self.Spawn Building`)
      (`self.K2_DestroyActor`))))

(fn `CheckingBuildingPlaced`
  (params (BuildingType :type "Actor Object Reference"))
  (bind _returnvalue (+ (`/Game/GameMode/GS_Builder_Base.CurrentWorkers` (`self.As GS Builder Base`)) 4))
  (set `self.Building Type` BuildingType)
  (`|ExecutionSequence`
    (:`then_0`
      ;[1 1 1] checks if house
      (if (`self.ActorHasTag` (`self.Building Type`) "House")
        (bind _asgs_builder_base (cast `/Game/GameMode/GS_Builder_Base` (`GameplayStatics.GetGameState`)))
        (set `self.As GS Builder Base` _asgs_builder_base)
        (`GameplayStatics.GetActorOfClass` "/Game/GameObjects/Objects/Placeable_Base_asset.Placeable_Base_asset_C")
        (bind _ashouse (cast `/Game/GameObjects/Objects/Apartment/House` (`self.Building Type`)))
        (if (`/Game/GameObjects/Objects/Placeable_Base_asset.IsUpgraded` _ashouse)
          (set `/Game/GameMode/GS_Builder_Base.CurrentWorkers` (- _returnvalue 2) (`self.As GS Builder Base`))
          (`self.SetPlacementModeEnabled` false)
          (else
            (set `/Game/GameMode/GS_Builder_Base.CurrentWorkers` _returnvalue (`self.As GS Builder Base`))
            (`self.SetPlacementModeEnabled` false)))))
    (:`then_1`
      ;[1 1 1] checks if shop removes workers and updates total amount of shops
      (if (`self.ActorHasTag` (`self.Building Type`) "Shop")
        (bind _asgs_builder_base_2 (cast `/Game/GameMode/GS_Builder_Base` (`GameplayStatics.GetGameState`)))
        (set `/Game/GameMode/GS_Builder_Base.NumberOfShops` (+ (`/Game/GameMode/GS_Builder_Base.CurrentWorkers` _asgs_builder_base_2) 1) (`self.As GS Builder Base`))
        (`self.SetPlacementModeEnabled` false)))
    (:`then_2`
      ;[1 1 1] checks if Power
      (if (`self.ActorHasTag` (`self.Building Type`) "Power")
        (bind _asgs_builder_base_3 (cast `/Game/GameMode/GS_Builder_Base` (`GameplayStatics.GetGameState`)))
        (set `/Game/GameMode/GS_Builder_Base.CurrentPower` (+ (`/Game/GameMode/GS_Builder_Base.CurrentPower` _asgs_builder_base_3) 5) _asgs_builder_base_3)
        (set `/Game/GameMode/GS_Builder_Base.TotalPower` (+ (`/Game/GameMode/GS_Builder_Base.TotalPower` _asgs_builder_base_3) 5) _asgs_builder_base_3)
        (`self.SetPlacementModeEnabled` false)))
    (:`then_3`
      ;[1 1 1] Checks if nature
      (if (`self.ActorHasTag` (`self.Building Type`) "Nature")
        (cast `/Game/GameMode/GS_Builder_Base` (`GameplayStatics.GetGameState`))
        (`self.SetPlacementModeEnabled` false)))))

(fn `SetPlacementModeEnabled`
  (params (isEnabled :type Boolean))
  (bind _placeableactor (`self.placeableActor`))
  ;[1 1 1] Set placement mode and turns off clickable component
  (if (== isEnabled (`self.placementModeActive`))
    (return)
    (else
      (bind _output_get (set `self.placementModeActive` isEnabled))
      (if _output_get
        (`self.UpdatesBuildingType`)
        (else
          (`/Engine/EditorBlueprintResources/StandardMacros.IsValid` _placeableactor
            (:`Is Valid`
              (`self.K2_DestroyActor` _placeableactor))))))))

(fn `Spawn Building`
  (locals (SpawnedActor :type "/Game/GameObjects/Objects/Placeable_Base_asset Object Reference"))
  (bind _spawnedactor (`local.SpawnedActor`))
  (bind _placeableactor (`self.placeableActor`))
  (bind _returnvalue (`self.GetComponentByClass` (`self.placeableActor`) "/Game/GameObjects/Components/PlaceablesComponent.PlaceablesComponent_C"))
  ;[1 1 1] Spawns Building
  (`/Engine/EditorBlueprintResources/StandardMacros.IsValid` _returnvalue
    (:`Is Valid`
      (if (`/Game/GameObjects/Components/PlaceablesComponent.IsplacementValid` _returnvalue)
        (bind _returnvalue_2 (`|SpawnActorFromClass` (`self.placeableActorType`) (`self.GetTransform` _placeableactor) "AlwaysSpawn" "MultiplyWithRoot" null 0 "False" 0 null))
        (set `local.SpawnedActor` _returnvalue_2)
        (bind _returnvalue_3 (`GameplayStatics.GetActorOfClass` "/Game/GameObjects/GridManager/GridManager.GridManager_C"))
        (bind _outgridcell (`/Game/GameObjects/GridManager/GridManager.GetNearestGridCell` _returnvalue_3 (`self.K2_GetActorLocation` _placeableactor)))
        (set `/Game/GameObjects/Objects/Placeable_Base_asset.gridcell` _outgridcell (`local.SpawnedActor`))
        (`/Engine/EditorBlueprintResources/StandardMacros.IsValid` (`local.SpawnedActor`)
          (:`Is Valid`
            (`/Game/GameObjects/GridManager/GridCell.SetOccupyed` _outgridcell (`/Game/GameObjects/Objects/Placeable_Base_asset.BuildingType` (`local.SpawnedActor`)) (`local.SpawnedActor`) true)
            (set `/Game/GameObjects/Objects/Placeable_Base_asset.bIsPlaced` true (`local.SpawnedActor`))
            ;;[1 1 1] road manager
            (bind _asroad_tile (cast `/Game/GameObjects/Objects/Road/RoadTile` (`local.SpawnedActor`))
              (:`then`
                (bind _returnvalue_4 (`GameplayStatics.GetActorOfClass` "/Game/GameObjects/Objects/Road/RoadManager.RoadManager_C"))
                (`/Game/GameObjects/Objects/Road/RoadManager.AddRoadTile` _returnvalue_4 _asroad_tile))
              (:`CastFailed`
                _))
            ;;[1 1 1] ChecksCost
            (bind _asgm_builder_base (cast `/Game/GameMode/GM_Builder_Base` (`GameplayStatics.GetGameMode`)))
            (`/Game/GameMode/GM_Builder_Base.BuyingObject` _asgm_builder_base (`/Game/GameObjects/Objects/Placeable_Base_asset.CostOfObjects` _spawnedactor) (`/Game/GameObjects/Objects/Placeable_Base_asset.WorkersNeeded` _spawnedactor) (`/Game/GameObjects/Objects/Placeable_Base_asset.PowerDrain` _spawnedactor) (`/Game/GameObjects/Objects/Placeable_Base_asset.PollutionCost` _spawnedactor))
            (`self.CheckingBuildingPlaced` (`local.SpawnedActor`))))))))

(fn `UpdatePlacement`
  (bind (_worldlocation _worlddirection) (`self.DeprojectMousePositionToWorld`))
  (bind _placeableactor (`self.placeableActor`))
  ;[1 1 1] Sets Spawned Actor To Mouse Locaction and snaps to grid
  (bind _outhit (`KismetSystemLibrary.LineTraceSingle` _worldlocation (+ _worldlocation (* _worlddirection 10000.0)) "TraceTypeQuery3"))
  (bind (_bblockinghit _binitialoverlap _time _distance _location) (`GameplayStatics.BreakHitResult` _outhit))
  (if _bblockinghit
    (bind _returnvalue (`GameplayStatics.GetActorOfClass` "/Game/GameObjects/GridManager/GridManager.GridManager_C"))
    (bind _outputvector (`/Game/GameObjects/GridManager/GridManager.GetNearestGridPlot` _returnvalue _location))
    (`/Engine/EditorBlueprintResources/StandardMacros.IsValid` _placeableactor
      (:`Is Valid`
        (`self.K2_SetActorLocation` _placeableactor _outputvector false false)))))

(fn `UpdatesBuildingType`
  (bind _returnvalue (`|SpawnActorFromClass` (`self.placeableActorType`) (`KismetMathLibrary.MakeTransform` (0.0 0.0 -1000000.0)) "Undefined" "MultiplyWithRoot" null 0 "False" 0 null))
  (bind _output_get (set `self.placeableActor` _returnvalue))
  (`/Engine/EditorBlueprintResources/StandardMacros.IsValid` _output_get
    (:`Is Valid`
      (bind _returnvalue_2 (`self.GetComponentByClass` _output_get "/Game/GameObjects/Components/BP_ClickAbleComponent.BP_ClickAbleComponent_C"))
      (`/Engine/EditorBlueprintResources/StandardMacros.IsValid` _returnvalue_2
        (:`Is Valid`
          (`/Game/GameObjects/Components/BP_ClickAbleComponent.InplacementMode` _returnvalue_2))
        (:`Is Not Valid`
          _))
      (bind _returnvalue_3 (`AddComponent|NODE_AddPlaceablesComponent-0` :`self` _output_get))
      (`/Game/GameObjects/Components/PlaceablesComponent.UpdateState` _returnvalue_3))))

(fn `updateWorkerCount`
  (params (AddedWorkers :type Integer))
  (bind _asgs_builder_base (cast `/Game/GameMode/GS_Builder_Base` (`GameplayStatics.GetGameState`)))
  (set `self.As GS Builder Base` _asgs_builder_base)
  (bind _returnvalue (`GameplayStatics.GetActorOfClass` "/Game/GameObjects/Objects/Placeable_Base_asset.Placeable_Base_asset_C"))
  (set `/Game/GameMode/GS_Builder_Base.CurrentWorkers` (+ (`/Game/GameObjects/Objects/Placeable_Base_asset.WorkersGiven` _returnvalue) AddedWorkers) (`self.As GS Builder Base`))
  (`self.SetPlacementModeEnabled` false))

(fn `UserConstructionScript`)
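; BP_ClickAbleComponent is an actor component that makes its owning actor clickable and highlights it on mouse hover.
; On BeginPlay it binds the owner's click event and the cursor-over events of the owner's static mesh.
; Hover toggles the mesh's render custom depth, while each click flips a clicked state that swaps the mesh material between green and red.
; An InplacementMode event destroys the component.
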(event `self.ReceiveBeginPlay`
  (bind _returnvalue (`self.GetOwner`))
  (bind _returnvalue_2 (`Actor.GetComponentByClass` _returnvalue "/Script/Engine.StaticMeshComponent"))
  ;[1 1 1] Add a clickable component to an actor
  (add `Actor.OnClicked` _returnvalue (delegate `OnMouseClicked`))
  (`/Engine/EditorBlueprintResources/StandardMacros.IsValid` _returnvalue_2
    (:`Is Valid`
      (set `self.StaticMeshRef` _returnvalue_2)
      (add `PrimitiveComponent.OnBeginCursorOver` _returnvalue_2 (delegate `OnMouseHover`))
      (add `PrimitiveComponent.OnEndCursorOver` _returnvalue_2 (delegate `onMouseHoverEnd`)))))

(event `onMouseHoverEnd`
  (params (TouchedComponent :type "PrimitiveComponent Object Reference"))
  ;[1 1 1] Add a clickable component to an actor
  (`PrimitiveComponent.SetRenderCustomDepth` (`self.StaticMeshRef`) false))

(event `OnMouseClicked`
  (params (TouchedActor :type "Actor Object Reference") (ButtonPressed :type "Key Structure" :default "None"))
  ;[1 1 1] Add a clickable component to an actor
  (bind _output_get (set `self.isClicked` (not (`self.isClicked`))))
  (`/Engine/EditorBlueprintResources/StandardMacros.IsValid` (`self.StaticMeshRef`)
    (:`Is Valid`
      (if _output_get
        (`PrimitiveComponent.SetMaterial` (`self.StaticMeshRef`) 0 "/Game/Materials/Green.Green")
        (else
          (`PrimitiveComponent.SetMaterial` (`self.StaticMeshRef`) 0 "/Game/Materials/Red.Red"))))))

(event `OnMouseHover`
  (params (TouchedComponent :type "PrimitiveComponent Object Reference"))
  ;[1 1 1] Add a clickable component to an actor
  (`PrimitiveComponent.SetRenderCustomDepth` (`self.StaticMeshRef`) true))

(event `InplacementMode`
  ;[1 1 1] destroys component
  (`self.K2_DestroyComponent`))
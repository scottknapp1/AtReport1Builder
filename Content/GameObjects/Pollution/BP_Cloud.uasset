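; Pollution cloud actor that shows the pollution level as the density of a Heterogeneous Volume.
; On BeginPlay it binds to the pollution change event of GM_Builder_Base and puts a dynamic instance of its cloud material on the volume.
; Its update event linearly scales the new pollution value into the material's Density Scale parameter.
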(event `self.ReceiveBeginPlay`
  ;[1 1 1] set material for cloud
  (bind _asgm_builder_base (cast `/Game/GameMode/GM_Builder_Base` (`GameplayStatics.GetGameMode`)))
  (add `/Game/GameMode/GM_Builder_Base.OnPollutionChange` _asgm_builder_base (`|CreateDelegate` :!event `UpdateCloudMaterial`))
  (bind _returnvalue (`PrimitiveComponent.CreateDynamicMaterialInstance` (`self.HeterogeneousVolume`) 0 (`self.CloudMaterial`) "None"))
  (bind _output_get (set `self.DynamicMaterialInstance` _returnvalue))
  (`PrimitiveComponent.SetMaterial` (`self.HeterogeneousVolume`) 0 _output_get))

(event `UpdateCloudMaterial`
  (params (NewPollutionValue :type Integer))
  ;[1 1 1] Updates Cloud density
  (`MaterialInstanceDynamic.SetScalarParameterValue` (`self.DynamicMaterialInstance`) "Density Scale" (* (`KismetMathLibrary.Conv_IntToDouble` NewPollutionValue) 0.002)))

(fn `UserConstructionScript`)
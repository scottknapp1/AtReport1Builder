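; Base game mode for a builder game that handles buying objects against money, worker, power and pollution totals.
; BuyingObject runs three affordability checks in sequence, each reading the current totals from GS_Builder_Base.
; If all pass, it deducts money, workers and power, adds pollution, then broadcasts OnPollutionChange with the new total.
; A failed check silently skips the purchase, and pollution is never a limit.
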(fn `BuyingObject`
  (params (ObjectCost :type Integer) (ObjectWorkers :type Integer) (ObjectivePower :type Integer) (ObjectPolution :type Integer))
  (bind _canafford (`self.HaveEnoughMoney` ObjectCost))
  (if _canafford
    (bind _canafford_2 (`self.HaveEnoughWorkers` ObjectWorkers))
    (if _canafford_2
      (bind _canafford_3 (`self.HaveEnoughPower` ObjectivePower))
      (if _canafford_3
        (bind _asgs_builder_base (cast `/Game/GameMode/GS_Builder_Base` (`GameplayStatics.GetGameState`)))
        (set `/Game/GameMode/GS_Builder_Base.CurrentMoney` (- (`/Game/GameMode/GS_Builder_Base.CurrentMoney` _asgs_builder_base) ObjectCost) _asgs_builder_base)
        (set `/Game/GameMode/GS_Builder_Base.CurrentWorkers` (- (`/Game/GameMode/GS_Builder_Base.CurrentWorkers` _asgs_builder_base) ObjectWorkers) _asgs_builder_base)
        (set `/Game/GameMode/GS_Builder_Base.CurrentPower` (- (`/Game/GameMode/GS_Builder_Base.CurrentPower` _asgs_builder_base) ObjectivePower) _asgs_builder_base)
        (bind _output_get (set `/Game/GameMode/GS_Builder_Base.CurrentPollution` (+ (`/Game/GameMode/GS_Builder_Base.CurrentPollution` _asgs_builder_base) ObjectPolution) _asgs_builder_base))
        (`self.OnPollutionChange` _output_get)))))

(fn `HaveEnoughMoney`
  (params (ObjectValue :type Integer))
  (returns (canAfford :type Boolean))
  (bind _asgs_builder_base (cast `/Game/GameMode/GS_Builder_Base` (`GameplayStatics.GetGameState`)))
  (return (<= ObjectValue (`/Game/GameMode/GS_Builder_Base.CurrentMoney` _asgs_builder_base))))

(fn `HaveEnoughPower`
  (params (PowerNeeded :type Integer))
  (returns (canAfford :type Boolean))
  (bind _asgs_builder_base (cast `/Game/GameMode/GS_Builder_Base` (`GameplayStatics.GetGameState`)))
  (return (>= (`/Game/GameMode/GS_Builder_Base.CurrentPower` _asgs_builder_base) PowerNeeded)))

(fn `HaveEnoughWorkers`
  (params (WorkersNeeded :type Integer))
  (returns (canAfford :type Boolean))
  (bind _asgs_builder_base (cast `/Game/GameMode/GS_Builder_Base` (`GameplayStatics.GetGameState`)))
  (return (>= (`/Game/GameMode/GS_Builder_Base.CurrentWorkers` _asgs_builder_base) WorkersNeeded)))

(fn `UserConstructionScript`)